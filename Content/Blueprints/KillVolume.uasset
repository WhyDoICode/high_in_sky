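; Kill volume that sends the player back to a checkpoint when they enter its box.
; On overlap with BP_Player, it shows the WI_Dead widget for a short delay, then removes it.
; If the player has a valid CheckPoint, it calls that checkpoint's Restor and moves the player just above it.
; Otherwise it moves the player to a hard-coded fallback world location.
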(event `self.Box.OnComponentBeginOverlap`
  (params (OverlappedComponent :type "PrimitiveComponent Object Reference") (OtherActor :type "Actor Object Reference") (OtherComp :type "PrimitiveComponent Object Reference") (OtherBodyIndex :type Integer) (bFromSweep :type Boolean) (SweepResult :type "HitResult Structure (by ref)"))
  (bind _checkpoint (`/Game/Resources/Blueprints/BP_Player.CheckPoint` (`self.As BP Player`)))
  (bind (_returnvalue_x _returnvalue_y _returnvalue_z) (`KismetMathLibrary.BreakVector` (`self.K2_GetActorLocation` _checkpoint)))
  (bind _asbp_player (cast `/Game/Resources/Blueprints/BP_Player` OtherActor))
  (set `self.As BP Player` _asbp_player)
  (bind _returnvalue (`|CreateWidget` "/Game/WI_Dead.WI_Dead_C"))
  (`UserWidget.AddToViewport` _returnvalue 0)
  (`KismetSystemLibrary.Delay` 2.0)
  (`Widget.RemoveFromParent` _returnvalue)
  (`/Engine/EditorBlueprintResources/StandardMacros.IsValid` _checkpoint
    (:`Is Valid`
      (`/Game/Blueprints/Checkpoint.Restor` _checkpoint)
      (`self.K2_SetActorLocation` (`self.As BP Player`) (`KismetMathLibrary.MakeVector` _returnvalue_x _returnvalue_y (+ _returnvalue_z 200.0)) false false))
    (:`Is Not Valid`
      (`self.K2_SetActorLocation` (`self.As BP Player`) (5835.0 -9470.0 2385.0) false false))))

(fn `UserConstructionScript`)
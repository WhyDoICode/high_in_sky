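; Checkpoint actor that spins slowly until the player activates it, then registers itself as that player's checkpoint.
; A box overlap with BP_Player fires once, stopping the rotation, setting the player's CheckPoint reference and playing a powerup sound.
; A Restor event prints a debug message and replaces actors in the Restore array with fresh same-class spawns at their current transforms, editing the array while looping over it.
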(event `self.ReceiveTick`
  (params (DeltaSeconds :type "Float (single-precision)"))
  (bind (_returnvalue_roll _returnvalue_pitch _returnvalue_yaw) (`KismetMathLibrary.BreakRotator` (`self.K2_GetActorRotation`)))
  (if (not (`self.Checked`))
    (`self.K2_SetActorRotation` (`KismetMathLibrary.MakeRotator` 0.0 0.0 (+ _returnvalue_yaw 0.4)))))

(event `self.Box.OnComponentBeginOverlap`
  (params (OverlappedComponent :type "PrimitiveComponent Object Reference") (OtherActor :type "Actor Object Reference") (OtherComp :type "PrimitiveComponent Object Reference") (OtherBodyIndex :type Integer) (bFromSweep :type Boolean) (SweepResult :type "HitResult Structure (by ref)"))
  (bind _asbp_player (cast `/Game/Resources/Blueprints/BP_Player` OtherActor))
  (`/Engine/EditorBlueprintResources/StandardMacros.DoOnce` false
    (:`Completed`
      (set `self.Checked` true)
      (set `/Game/Resources/Blueprints/BP_Player.CheckPoint` self _asbp_player)
      (`GameplayStatics.PlaySound2D` "/Game/Ultimate_SFX/UI_Item_Sounds_HD_Remake/Wavs/Powerup_upgrade_3.Powerup_upgrade_3" 1.0 1.0 0.0 null null))))

(event `Restor`
  (bind _restore (`self.Restore`))
  (`KismetSystemLibrary.PrintString` "Hello")
  (for _array_element (`self.Restore`)
    (bind _returnvalue (`|SpawnActorFromClass` (`GameplayStatics.GetObjectClass` _array_element) (`self.GetTransform` _array_element) "AlwaysSpawn" "MultiplyWithRoot" null null))
    (`KismetArrayLibrary.Array_Add` _restore _returnvalue)
    (`self.K2_DestroyActor` _array_element)
    (`KismetArrayLibrary.Array_RemoveItem` _restore _array_element)))

(fn `UserConstructionScript`)
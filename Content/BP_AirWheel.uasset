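; BP_AirWheel is a powerable wheel actor that acts as a win trigger when it receives power.
; PowerChanged, when IsPowered is true, latches Condition and calls Won on the player's BP_Player; nothing here clears Condition.
; While Condition is set, Tick adds a fixed roll step each frame, so the spin is frame-rate dependent.
; The Interact_1 event is empty.
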(event `self.ReceiveTick`
  (params (DeltaSeconds :type "Float (single-precision)"))
  (bind (_returnvalue_roll _returnvalue_pitch _returnvalue_yaw) (`KismetMathLibrary.BreakRotator` (`self.K2_GetActorRotation`)))
  (`parent.ReceiveTick` DeltaSeconds)
  (if (`self.Condition`)
    (`self.K2_SetActorRotation` (`KismetMathLibrary.MakeRotator` (+ _returnvalue_roll 2.0) _returnvalue_pitch _returnvalue_yaw) true)))

(event `self.Power changed`
  (if (`self.Is powered?`)
    (set `self.Condition` true)
    (bind _asbp_player (cast `/Game/Resources/Blueprints/BP_Player` (`GameplayStatics.GetPlayerCharacter` 0)))
    (`/Game/Resources/Blueprints/BP_Player.Won` _asbp_player)))

(event `Interact_1`)

(fn `UserConstructionScript`
  (`parent.UserConstructionScript`))
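; BP_ElectricDoor is a door that rotates open on interaction, consuming or checking a key in BP_Player's inventory if one is assigned.
; A missing key shows a HUD notification; otherwise a DoOnce plays the opening sound and a Timeline lerps the actor to IntendedRotation.
; PowerChanged triggers the interaction when IsPowered is true.
; A Rever event reverses the Timeline but is not called within this Blueprint.
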(event `Interact_1`
  (`/Engine/EditorBlueprintResources/StandardMacros.IsValid` (`self.Key`)
    (:`Is Valid`
      (bind _asbp_player (cast `/Game/Resources/Blueprints/BP_Player` (`GameplayStatics.GetPlayerCharacter` 0)))
      (bind _newparam (`/Game/Resources/Blueprints/BP_Player.UseInventory` _asbp_player (`self.Key`)))
      (if _newparam
        (`/Engine/EditorBlueprintResources/StandardMacros.DoOnce` false :!label _label
          (:`Completed`
            (`GameplayStatics.PlaySound2D` "/Game/Ultimate_SFX/Survival_Sound_Kit_HD_Remake/Wavs/Door_Open.Door_Open" 1.0 1.0 0.0 null null)
            (set `self.Rotation` (`self.K2_GetActorRotation`))
            (bind (_direction _newtrack_0) (`Timeline|Timeline` :!via `PlayFromStart` :!label _label_2)
              (:`Update`
                (`self.K2_SetActorRotation` (`KismetMathLibrary.RLerp` (`self.Rotation`) (`self.IntendedRotation`) _newtrack_0))))))
        (else
          (`/Game/ProHUDV2_Horror/Blueprints/Libraries/BPi_HUDManagerV2_H.AddPickupNotification_H` (`/Game/ProHUDV2_Horror/Blueprints/Libraries/BP_PHV2_Functions_H.GetHUDManager_H`) "f" (make `/Game/ProHUDV2_Horror/Blueprints/Structs/S_PickupNoti_Info_H` 0 2.0 (struct :`Transform` (struct :`Translation` (0.0 0.0) :`Scale` (1.0 1.0) :`Shear` (0.0 0.0)) :`IconColor` (struct)) "No Key Found")))))
    (:`Is Not Valid`
      (goto _label))))

(event `Rever`
  (goto _label_2 :!via `Reverse`))

(event `self.Power changed`
  (if (`self.Is powered?`)
    (`self.Interact_1`)))

(fn `UserConstructionScript`
  (`parent.UserConstructionScript`))
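; BP_Pickable is a pickup actor that goes into the player's inventory when interacted with.
; Its Interact event casts the player character to BP_Player and passes itself to AddToInventory.
; Instead of being destroyed, the actor is moved to the world origin.
; It then posts a timed HUD pickup notification showing its ItemName and plays a 2D collect sound.
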(event `self.Interact`
  (bind _item_name (`self.Item Name`))
  (bind _asbp_player (cast `/Game/Resources/Blueprints/BP_Player` (`GameplayStatics.GetPlayerCharacter` 0)))
  (`/Game/Resources/Blueprints/BP_Player.AddToInventory` _asbp_player self)
  (`self.K2_SetActorLocation` (0.0 0.0 0.0))
  (`/Game/Resources/External/ProHUDV2_Horror/Blueprints/Libraries/BPi_HUDManagerV2_H.AddPickupNotification_H` (`/Game/Resources/External/ProHUDV2_Horror/Blueprints/Libraries/BP_PHV2_Functions_H.GetHUDManager_H`) _item_name (make `/Game/Resources/External/ProHUDV2_Horror/Blueprints/Structs/S_PickupNoti_Info_H` 0 3.0 (struct :`Transform` (struct :`Translation` (0.0 0.0) :`Scale` (1.0 1.0) :`Shear` (0.0 0.0)) :`IconColor` (struct)) (`KismetTextLibrary.Conv_StringToText` _item_name) (make `/Game/Resources/External/ProHUDV2_Horror/Blueprints/Structs/S_TextInfo_H` false)))
  (`GameplayStatics.PlaySound2D` "/Game/Resources/Sounds/SFX/UISounds/Wavs/Collect_star_5.Collect_star_5" 1.0 1.0 0.0 null null))

(fn `UserConstructionScript`
  (`parent.UserConstructionScript`))
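; BridgeFall is a scripted collapse in which wooden-sounding pieces break loose and fall when the player enters trigger boxes.
; One box switches on physics for a fort wall mesh with a 2D break sound.
; The other drops three static meshes and a mine track barrier in a delayed sequence, playing the sound at each piece.
; Both triggers respond only to BP_Player and fire once through DoOnce.
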(event `self.Box.OnComponentBeginOverlap`
  (params (OverlappedComponent :type "PrimitiveComponent Object Reference") (OtherActor :type "Actor Object Reference") (OtherComp :type "PrimitiveComponent Object Reference") (OtherBodyIndex :type Integer) (bFromSweep :type Boolean) (SweepResult :type "HitResult Structure (by ref)"))
  (cast `/Game/Resources/Blueprints/BP_Player` OtherActor)
  (`/Engine/EditorBlueprintResources/StandardMacros.DoOnce` false
    (:`Completed`
      (`PrimitiveComponent.SetSimulatePhysics` (`self.SM_Bld_Fort_Wall_02`) true)
      (`GameplayStatics.PlaySound2D` "/Game/Resources/Sounds/SFX/WoodAndWalk/Wavs/Wood_Break_10_Cue.Wood_Break_10_Cue" 0.7 1.0 0.0 null null))))

(event `self.Box1.OnComponentBeginOverlap`
  (params (OverlappedComponent :type "PrimitiveComponent Object Reference") (OtherActor :type "Actor Object Reference") (OtherComp :type "PrimitiveComponent Object Reference") (OtherBodyIndex :type Integer) (bFromSweep :type Boolean) (SweepResult :type "HitResult Structure (by ref)"))
  (cast `/Game/Resources/Blueprints/BP_Player` OtherActor)
  (`/Engine/EditorBlueprintResources/StandardMacros.DoOnce` false
    (:`Completed`
      (`PrimitiveComponent.SetSimulatePhysics` (`self.StaticMesh`) true)
      (`GameplayStatics.PlaySoundAtLocation` "/Game/Resources/Sounds/SFX/WoodAndWalk/Wavs/Wood_Break_10_Cue.Wood_Break_10_Cue" (`SceneComponent.K2_GetComponentLocation` (`self.StaticMesh`)) (struct) 0.4 1.0 0.0 null null null null)
      (`KismetSystemLibrary.Delay` 0.8)
      (`PrimitiveComponent.SetSimulatePhysics` (`self.StaticMesh1`) true)
      (`GameplayStatics.PlaySoundAtLocation` "/Game/Resources/Sounds/SFX/WoodAndWalk/Wavs/Wood_Break_10_Cue.Wood_Break_10_Cue" (`SceneComponent.K2_GetComponentLocation` (`self.StaticMesh1`)) (struct) 0.4 1.0 0.0 null null null null)
      (`KismetSystemLibrary.Delay` 0.8)
      (`PrimitiveComponent.SetSimulatePhysics` (`self.StaticMesh2`) true)
      (`GameplayStatics.PlaySoundAtLocation` "/Game/Resources/Sounds/SFX/WoodAndWalk/Wavs/Wood_Break_10_Cue.Wood_Break_10_Cue" (`SceneComponent.K2_GetComponentLocation` (`self.StaticMesh2`)) (struct) 0.4 1.0 0.0 null null null null)
      (`KismetSystemLibrary.Delay` 0.8)
      (`PrimitiveComponent.SetSimulatePhysics` (`self.SM_Env_Mine_Track_Barrier_01`) true)
      (`GameplayStatics.PlaySoundAtLocation` "/Game/Resources/Sounds/SFX/WoodAndWalk/Wavs/Wood_Break_10_Cue.Wood_Break_10_Cue" (`SceneComponent.K2_GetComponentLocation` (`self.SM_Env_Mine_Track_Barrier_01`)) (struct) 0.4 1.0 0.0 null null null null))))

(fn `UserConstructionScript`)
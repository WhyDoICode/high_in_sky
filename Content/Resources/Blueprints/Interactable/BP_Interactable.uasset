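; BP_Interactable is an interactable actor that flags its mesh for highlighting when the player is near.
; Every Tick it compares its distance to the player character against a threshold (NewVar) and toggles the Mesh's custom depth rendering.
; BeginPlay casts the root's child components to static meshes but does nothing with the result.
; The Interact event is an empty stub.
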(event `self.ReceiveBeginPlay`
  (for _array_element (`SceneComponent.GetChildrenComponents` (`self.DefaultSceneRoot`) false)
    (cast `StaticMeshComponent` _array_element)))

(event `self.ReceiveTick`
  (params (DeltaSeconds :type "Float (single-precision)"))
  (bind _mesh (`self.Mesh`))
  (if (< (`KismetMathLibrary.Vector_Distance` (`self.K2_GetActorLocation` (`GameplayStatics.GetPlayerCharacter` 0)) (`self.K2_GetActorLocation`)) (`self.NewVar`))
    (`PrimitiveComponent.SetRenderCustomDepth` _mesh true)
    (else
      (`PrimitiveComponent.SetRenderCustomDepth` _mesh false))))

(event `Interact`)

(fn `UserConstructionScript`)
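; BP_Paper is an interactable paper note that the player can read.
; On Interact it creates a WI_TextReader widget filled with its Description and Titles values and adds it to the viewport.
; It also plays a paper foley sound and a second sound from its Sound variable.
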(event `self.Interact`
  (bind _returnvalue (`|CreateWidget` "/Game/Resources/Widgets/WI_TextReader.WI_TextReader_C" null (`self.Description`) (`self.Titles`)))
  (`UserWidget.AddToViewport` _returnvalue 0)
  (`GameplayStatics.PlaySound2D` "/Game/Resources/Sounds/SFX/WoodAndWalk/Wavs/Paper_Foley_5.Paper_Foley_5" 1.0 1.0 0.0 null null)
  (`GameplayStatics.PlaySound2D` (`self.Sound`) 1.0 1.0 0.0 null null))

(fn `UserConstructionScript`
  (`parent.UserConstructionScript`))
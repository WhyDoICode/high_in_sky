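; BP_Enemy is an electricity-powered child actor that damages the Howizter boss it is attached to.
; When PowerChanged reports power, it casts its attach parent to BP_Boss_Howizter and applies a fixed health decrease through BossBehavior, with debug prints.
; On power loss it deactivates Fire and reverses a timeline that modulates audio volume and pitch.
; The flamethrower's activation and forward timeline nodes are disconnected.
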(event `self.Power changed`
  (bind _audio (`self.Audio`))
  ;[0 0 0] Activate flamethrower
  (`parent.Power changed`)
  (if (`self.Is powered?`)
    (`KismetSystemLibrary.PrintString` "Hello")
    (bind _asbp_boss_howizter (cast `/Game/Resources/Blueprints/BossExamples/BP_Boss_Howizter` (`self.GetAttachParentActor`)))
    (`KismetSystemLibrary.PrintString` "GGG")
    (`/Game/Resources/Blueprints/BossBase/BPC_Boss_Behavior.DecreaseHealth` (`/Game/Resources/Blueprints/BossBase/BP_Boss_Base.Boss Behavior` _asbp_boss_howizter) 2500.0)
    (else
      (`ActorComponent.Deactivate` (`self.Fire`))
      ;[0 0 0] Flames sound modulation
      (bind (_direction _newtrack_0) (`Timeline|Timeline_0` :!via `Reverse`)
        (:`Update`
          (`AudioComponent.SetVolumeMultiplier` _audio _newtrack_0)
          (`AudioComponent.SetPitchMultiplier` _audio (`KismetMathLibrary.Lerp` 2.0 1.0 _newtrack_0)))))))

(fn `UserConstructionScript`
  (`parent.UserConstructionScript`))
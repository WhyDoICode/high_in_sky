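; Generator Blueprint for the electricity system that the player toggles to produce power.
; Activation flips GeneratesPower, updates all electrical actors, and switches the smoke effect and generator animation.
; A start-up timeline fades the motor sound's volume and pitch in, and reverses on stop.
; A second timeline scales and rolls the mesh as vibration, weighted by start-up progress, though no wire in the graph starts it.
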(event `self.Player activated`
  (bind _motor_sound (`self.Motor Sound`))
  (bind _smoke (`self.Smoke`))
  ;[0 0 0] Turn generator on / off when player activates
  (bind _output_get (set `self.Generates power?` (not (`self.Generates power?`))))
  (`self.Update all electrical actors`)
  (if _output_get
    (`ActorComponent.Activate` _smoke false)
    (bind (_direction _newtrack_0) (`Timeline|Generator start up animation` :!label _label)
      (:`Update`
        (`AudioComponent.SetVolumeMultiplier` _motor_sound _newtrack_0)
        (`AudioComponent.SetPitchMultiplier` _motor_sound (`KismetMathLibrary.Lerp` 0.0 1.25 _newtrack_0))))
    (else
      (`ActorComponent.Deactivate` _smoke)
      (goto _label :!via `Reverse`))))

(fn `UserConstructionScript`
  (`parent.UserConstructionScript`))
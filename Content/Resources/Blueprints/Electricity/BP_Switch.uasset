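; BP_Switch is an electrical switch that the player activates to open or close a circuit.
; PlayerActivated plays or reverses a timeline, chosen by ClosedCircuit, which lerps the Switch component's pitch between 0 and 180 degrees.
; While the timeline value is near its top, each update sets ClosedCircuit true only at exactly full travel and calls UpdateAllElectricalActors.
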(event `self.Player activated`
  ;[0 0 0] Flip the switch and open / close the circuit when activated by the player
  (if (not (`self.Closed circuit?`))
    (bind (_direction _newtrack_0) (`Timeline|Switch animation` :!label _label)
      (:`Update`
        (`SceneComponent.K2_SetRelativeRotation` (`self.Switch`) (`KismetMathLibrary.MakeRotator` 0.0 (`KismetMathLibrary.Lerp` 0.0 180.0 _newtrack_0)) false false)
        (if (> _newtrack_0 0.95)
          (set `self.Closed circuit?` (== _newtrack_0 1.0))
          (`self.Update all electrical actors`))))
    (else
      (goto _label :!via `Reverse`))))

(fn `UserConstructionScript`
  (`parent.UserConstructionScript`))
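; Area damage ability that hits everything within a radius around its own location.
; On begin play it reads the radius from the X component of the ability info modifier and shows a circular telegraph of that size.
; When damage begins, it applies radial ability damage over the same radius from the actor's location and removes the telegraph.
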(event `self.ReceiveBeginPlay`
  (`parent.ReceiveBeginPlay`)
  (set `self.Radius` (.x (`.Modifier_68_9F6259774C70A5FB7DE538BB3C951747` (break `/Game/Resources/Blueprints/Structs/F_BossAbility` (`self.AbilityInfo`)))))
  (`self.TelegraphCircle` (`self.Radius`) (`self.K2_GetActorLocation`)))

(event `self.OnBeginDamage`
  (params (Duration :type "Float (double-precision)"))
  (`self.ApplyAbilityDamage` null (`self.K2_GetActorLocation`) true (`self.Radius`))
  (`self.RemoveTelegraph`))

(fn `UserConstructionScript`
  (`parent.UserConstructionScript`))
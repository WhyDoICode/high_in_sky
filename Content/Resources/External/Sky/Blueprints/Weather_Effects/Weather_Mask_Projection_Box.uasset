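; Placeable box for Ultra Dynamic Weather that masks snow/dust and wetness beneath occluding geometry inside its volume.
; A top-mounted orthographic scene capture renders depth to a lazily created, releasable render target, feeding a blurred brush material for the weather mask.
; The box registers with the weather actor at runtime and refreshes its mask in editor on construction.
; Point occlusion queries approximate the mask with upward traces, using more samples as blur radius grows.
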(event `self.ReceiveBeginPlay`
  (bind _returnvalue (`GameplayStatics.GetActorOfClass` "/Game/Resources/External/Sky/Blueprints/Ultra_Dynamic_Weather.Ultra_Dynamic_Weather_C"))
  (set `self.UDW` _returnvalue)
  (if (`/Game/Resources/External/Sky/Blueprints/Ultra_Dynamic_Weather.Initialized` (`self.UDW`))
    (if (not (`KismetArrayLibrary.Array_Contains` (`/Game/Resources/External/Sky/Blueprints/Ultra_Dynamic_Weather.All Weather Mask Projection Boxes` (`self.UDW`)) self))
      (if (`/Game/Resources/External/Sky/Blueprints/Ultra_Dynamic_Weather.Weather Mask Target in Use` (`self.UDW`))
        (`KismetArrayLibrary.Array_Add` (`/Game/Resources/External/Sky/Blueprints/Ultra_Dynamic_Weather.All Weather Mask Projection Boxes` (`self.UDW`)) self)
        (`/Game/Resources/External/Sky/Blueprints/Ultra_Dynamic_Weather.Draw Weather Mask Brush Target` (`self.UDW`) false)
        (else
          (`/Game/Resources/External/Sky/Blueprints/Ultra_Dynamic_Weather.Initialize Weather Mask Target` (`self.UDW`)))))))

(event `self.ReceiveEndPlay`
  (params (EndPlayReason :type "EEndPlayReason Enum" :default "Destroyed"))
  (if (`KismetArrayLibrary.Array_Contains` (`|MakeArray` "Destroyed" "RemovedFromWorld" :!type "EEndPlayReason Enum") EndPlayReason)
    (`/Engine/EditorBlueprintResources/StandardMacros.IsValid` (`self.UDW`)
      (:`Is Valid`
        (`/Game/Resources/External/Sky/Blueprints/Ultra_Dynamic_Weather.Report Removal of Drawing Actor` (`self.UDW`) self)))))

(fn `Force Update`
  (`self.Update Capture`)
  (`/Game/Resources/External/Sky/Blueprints/Ultra_Dynamic_Weather.Draw Weather Mask Brush Target` (`self.UDW`) false))

(fn `Recycle Render Target`
  (`/Engine/EditorBlueprintResources/StandardMacros.IsValid` (`self.Depth Render Target`)
    (:`Is Valid`
      (`KismetRenderingLibrary.ReleaseRenderTarget2D` (`self.Depth Render Target`))
      (set `self.Depth Render Target` null))))

(fn `Test Point Occlusion`
  (params (Location :type "Vector Structure") (Mode :type "/Game/Resources/External/Sky/Blueprints/Enum/UDS_DLWE_Mode Enum" :default "NewEnumerator0"))
  (returns (`In Volume` :type Boolean) (Occlusion :type "Float (double-precision)"))
  (locals (`Do Trace` :type Boolean :default false) (`Trace Hit` :type Boolean :default false) (`Total Occlusion` :type "Float (double-precision)") (`Number of Traces` :type Integer :default 0) (`9 Trace Vectors` :type "Array of Vector Structure") (`5 Trace Vectors` :type "Array of Vector Structure") (`1 Trace Vector` :type "Array of Vector Structure"))
  (bind _returnvalue (select `int` (`KismetMathLibrary.Clamp` (`KismetMathLibrary.FCeil` (/ (- (`self.Blur Radius`) 1.0) 80.0)) 0 2) :`0` (`local.1 Trace Vector`) :`1` (`local.5 Trace Vectors`) :`2` (`local.9 Trace Vectors`)))
  (bind _output_get (set `local.Do Trace` (and (< (.x (`KismetMathLibrary.Vector_GetAbs` (`KismetMathLibrary.InverseTransformLocation` (`self.GetTransform`) Location))) (.x (`self.Box Extent`))) (< (.y (`KismetMathLibrary.Vector_GetAbs` (`KismetMathLibrary.InverseTransformLocation` (`self.GetTransform`) Location))) (.y (`self.Box Extent`))) (< (.z Location) (`self.Top Height`)))))
  (if _output_get
    (set `local.Number of Traces` (`KismetArrayLibrary.Array_Length` _returnvalue))
    (for _array_element _returnvalue
      (bind _returnvalue_2 (+ (* _array_element (* (`self.Blur Radius`) 0.75)) (`local.Location`)))
      (bind (_outhit _returnvalue_3) (`KismetSystemLibrary.LineTraceSingleForObjects` (+ _returnvalue_2 (0.0 0.0 10.0)) (`KismetMathLibrary.MakeVector` (.x _returnvalue_2) (.y _returnvalue_2) (`self.Top Height`)) (`|MakeArray` "ObjectTypeQuery1" :!type "EObjectTypeQuery Enum") false (`self.Exclude Actors from Occlusion`) "None" true (struct :`R` 1.0 :`A` 1.0) (struct :`G` 1.0 :`A` 1.0) 0.2))
      (if _returnvalue_3
        (set `local.Total Occlusion` (+ (`local.Total Occlusion`) (/ 1.0 (`KismetMathLibrary.Conv_IntToDouble` (`local.Number of Traces`)))))))
    (set `local.Total Occlusion` (* (`local.Total Occlusion`) (select `/Game/Resources/External/Sky/Blueprints/Enum/UDS_DLWE_Mode` (`local.Mode`) :`NewEnumerator0` (`self.Mask Snow / Dust`) :`NewEnumerator1` (`self.Mask Wetness`)))))
  (return (`local.Do Trace`) (`local.Total Occlusion`)))

(fn `Update Capture`
  (`/Engine/EditorBlueprintResources/StandardMacros.IsValid` (`self.Depth Render Target`)
    (:`Is Valid`
      _)
    (:`Is Not Valid`
      (bind _returnvalue (`KismetRenderingLibrary.CreateRenderTarget2D` (`KismetMathLibrary.Clamp` (`KismetMathLibrary.FTrunc` (.x (/ (`self.Scaled Box Extent`) (`self.Capture Pixel Size`)))) 8 4000) (`KismetMathLibrary.Clamp` (`KismetMathLibrary.FTrunc` (.y (/ (`self.Scaled Box Extent`) (`self.Capture Pixel Size`)))) 8 4000) "RTF_R16f"))
      (set `self.Depth Render Target` _returnvalue)
      (set `TextureRenderTarget2D.AddressX` "TA_Clamp" _returnvalue)
      (set `TextureRenderTarget2D.AddressY` "TA_Clamp" _returnvalue)
      (set `SceneCaptureComponent2D.TextureTarget` (`self.Depth Render Target`) (`self.SceneCaptureComponent2D`))
      (`MaterialInstanceDynamic.SetTextureParameterValue` (`self.Brush_MID`) "Tex" (`self.Depth Render Target`))))
  (`SceneCaptureComponent2D.CaptureScene` (`self.SceneCaptureComponent2D`)))

(fn `UserConstructionScript`
  (bind _box (`self.Box`))
  (bind (_x _y) (`KismetMathLibrary.BreakVector2D` (`self.Brush Scale`)))
  (bind _returnvalue (/ (`KismetMathLibrary.GetAbsMax2D` (`self.Brush Scale`)) 2.0))
  ;[1 0.6154 0.2299] Actor Rotation, Preview Box Extent
  (`self.K2_SetActorRotation` (`KismetMathLibrary.MakeRotator` 0.0 0.0 (.yaw (`self.K2_GetActorRotation`))))
  (set `self.Yaw` (.yaw (`self.K2_GetActorRotation`)))
  (`/Engine/EditorBlueprintResources/StandardMacros.IsValid` _box
    (:`Is Valid`
      (`BoxComponent.SetBoxExtent` _box (`self.Box Extent`) false))
    (:`Is Not Valid`
      _))
  ;[0.8397 0.4791 1] Scene Capture 2D
  (`SceneComponent.K2_SetRelativeLocation` (`self.SceneCaptureComponent2D`) (`KismetMathLibrary.MakeVector` 0.0 0.0 (.z (`self.Box Extent`))) false false)
  (set `SceneCaptureComponent2D.OrthoWidth` (* (.x (`self.Scaled Box Extent`)) 2.0) (`self.SceneCaptureComponent2D`))
  (set `SceneCaptureComponent.HiddenActors` (`self.Exclude Actors from Occlusion`) (`self.SceneCaptureComponent2D`))
  ;[0.19 0.4583 0.1889 1 35] Brush Data
  (`|ExecutionSequence`
    (:`then_0`
      (`KismetArrayLibrary.Array_Clear` (`self.Corners`))
      (set `self.Brush Scale` (`KismetMathLibrary.Conv_VectorToVector2D` (* (`self.Scaled Box Extent`) 2.0)))
      (bind _output_get (set `self.Center Location` (`KismetMathLibrary.Conv_VectorToVector2D` (`self.K2_GetActorLocation`))))
      (set `self.Brush Location` (- _output_get (/ (`self.Brush Scale`) 2.0)))
      (set `self.Max Distance` (`KismetMathLibrary.Hypotenuse` _returnvalue _returnvalue))
      (for _index (range 4)
        (`KismetArrayLibrary.Array_Add` (`self.Corners`) (+ (`KismetMathLibrary.Conv_VectorToVector2D` (`self.K2_GetActorLocation`)) (`KismetMathLibrary.GetRotated2D` (* (`self.Brush Scale`) (select `int` _index :`0` (-1.0 -1.0) :`1` (1.0 1.0) :`2` (-1.0 1.0) :`3` (1.0 -1.0) :!type "Vector2D Structure")) (`self.Yaw`))))))
    (:`then_1`
      ;[1 0.5585 0.3036 1 35] Brush MID
      (`|ExecutionSequence`
        (:`then_0`
          (bind _returnvalue_2 (`KismetMaterialLibrary.CreateDynamicMaterialInstance` "/Game/Resources/External/Sky/Materials/Weather/Weather_Mask_ProjectionBox_Mat.Weather_Mask_ProjectionBox_Mat"))
          (set `self.Brush_MID` _returnvalue_2)
          (bind _output_get_2 (set `self.Top Height` (.z (`SceneComponent.K2_GetComponentLocation` (`self.SceneCaptureComponent2D`)))))
          (`MaterialInstanceDynamic.SetScalarParameterValue` (`self.Brush_MID`) "SceneCapture Height" _output_get_2)
          (`MaterialInstanceDynamic.SetScalarParameterValue` (`self.Brush_MID`) "Depth Range" (- (* (.z (`self.Scaled Box Extent`)) 2.0) 1.0))
          (`MaterialInstanceDynamic.SetScalarParameterValue` (`self.Brush_MID`) "Mask Snow Coverage" (`self.Mask Snow / Dust`))
          (`MaterialInstanceDynamic.SetScalarParameterValue` (`self.Brush_MID`) "Mask Wetness" (`self.Mask Wetness`))
          (`MaterialInstanceDynamic.SetScalarParameterValue` (`self.Brush_MID`) "Y Scale" (/ _x _y))
          (`MaterialInstanceDynamic.SetScalarParameterValue` (`self.Brush_MID`) "Blur Slope Snow" (`self.Blur Slope (Snow/Dust)`))
          (`MaterialInstanceDynamic.SetScalarParameterValue` (`self.Brush_MID`) "Blur Slope Wetness" (`self.Blur Slope (Wetness)`))
          (bind _returnvalue_3 (`GameplayStatics.GetActorOfClass` "/Game/Resources/External/Sky/Blueprints/Ultra_Dynamic_Weather.Ultra_Dynamic_Weather_C"))
          (`MaterialInstanceDynamic.SetScalarParameterValue` (`self.Brush_MID`) "Blur Radius" (`KismetMathLibrary.SafeDivide` (/ (`self.Blur Radius`) (/ (`KismetMathLibrary.BreakVector2D` (`self.Brush Scale`)) 20000.0)) (`KismetMathLibrary.Conv_IntToDouble` (`/Game/Resources/External/Sky/Blueprints/Ultra_Dynamic_Weather.Weather Mask Target Size` _returnvalue_3)))))
        (:`then_1`
          ;[0.4334 0.3801 1 1 35] Update UDW in Editor
          (if (not (`KismetSystemLibrary.IsPackagedForDistribution`))
            (bind _returnvalue_4 (`GameplayStatics.GetActorOfClass` "/Game/Resources/External/Sky/Blueprints/Ultra_Dynamic_Weather.Ultra_Dynamic_Weather_C"))
            (if (not (`/Game/Resources/External/Sky/Blueprints/Ultra_Dynamic_Weather.Runtime` _returnvalue_4))
              (set `/Game/Resources/External/Sky/Blueprints/Ultra_Dynamic_Weather.Editor Mask Target Root` (`self.K2_GetActorLocation`) _returnvalue_4)
              (`/Game/Resources/External/Sky/Blueprints/Ultra_Dynamic_Weather.Initialize Weather Mask Target` _returnvalue_4))))))))
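; Placeable brush actor for Ultra Dynamic Weather that draws a wetness and snow/dust mask into the weather mask target.
; Construction flattens rotation to yaw, derives footprint, corners and max distance from the transform, selects a gradient or shape texture, and packs mask amounts into red and green.
; In editor it re-centers and reinitializes the mask target.
; At play it registers with the weather actor, reporting removal when destroyed or unloaded.
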(event `self.ReceiveBeginPlay`
  (bind _returnvalue (`GameplayStatics.GetActorOfClass` "/Game/Resources/External/Sky/Blueprints/Ultra_Dynamic_Weather.Ultra_Dynamic_Weather_C"))
  (set `self.UDW` _returnvalue)
  (if (`/Game/Resources/External/Sky/Blueprints/Ultra_Dynamic_Weather.Initialized` (`self.UDW`))
    (if (not (`KismetArrayLibrary.Array_Contains` (`/Game/Resources/External/Sky/Blueprints/Ultra_Dynamic_Weather.All Weather Mask Brushes` (`self.UDW`)) self))
      (if (`/Game/Resources/External/Sky/Blueprints/Ultra_Dynamic_Weather.Weather Mask Target in Use` (`self.UDW`))
        (`KismetArrayLibrary.Array_Add` (`/Game/Resources/External/Sky/Blueprints/Ultra_Dynamic_Weather.All Weather Mask Brushes` (`self.UDW`)) self)
        (`/Game/Resources/External/Sky/Blueprints/Ultra_Dynamic_Weather.Draw Weather Mask Brush Target` (`self.UDW`) false)
        (else
          (`/Game/Resources/External/Sky/Blueprints/Ultra_Dynamic_Weather.Initialize Weather Mask Target` (`self.UDW`)))))))

(event `self.ReceiveEndPlay`
  (params (EndPlayReason :type "EEndPlayReason Enum" :default "Destroyed"))
  (if (`KismetArrayLibrary.Array_Contains` (`|MakeArray` "Destroyed" "RemovedFromWorld" :!type "EEndPlayReason Enum") EndPlayReason)
    (`/Engine/EditorBlueprintResources/StandardMacros.IsValid` (`self.UDW`)
      (:`Is Valid`
        (`/Game/Resources/External/Sky/Blueprints/Ultra_Dynamic_Weather.Report Removal of Drawing Actor` (`self.UDW`) self)))))

(fn `UserConstructionScript`
  (bind _returnvalue (/ (`KismetMathLibrary.GetAbsMax2D` (`self.Brush Scale`)) 2.0))
  (`self.K2_SetActorRotation` (`KismetMathLibrary.MakeRotator` 0.0 0.0 (.yaw (`self.K2_GetActorRotation`))))
  (set `self.Yaw` (.yaw (`self.K2_GetActorRotation`)))
  (set `self.Brush Scale` (* (`KismetMathLibrary.Conv_VectorToVector2D` (`self.GetActorScale3D`)) 1000.0))
  (`KismetArrayLibrary.Array_Clear` (`self.Corners`))
  (set `self.Brush Texture` (select `/Game/Resources/External/Sky/Blueprints/Enum/UDS_Weather_Mask_Brush` (`self.Brush`) :`NewEnumerator0` "/Game/Resources/External/Sky/Textures/Weather/Mask_Brushes/Brush_Radial.Brush_Radial" :`NewEnumerator1` "/Game/Resources/External/Sky/Textures/Weather/Mask_Brushes/Brush_Pyramid.Brush_Pyramid" :`NewEnumerator2` "/Game/Resources/External/Sky/Textures/Weather/Mask_Brushes/Brush_Square.Brush_Square" :`NewEnumerator3` "/Game/Resources/External/Sky/Textures/Weather/Mask_Brushes/Brush_Circle.Brush_Circle" :`NewEnumerator4` "/Game/Resources/External/Sky/Textures/Weather/Mask_Brushes/Brush_Falloff.Brush_Falloff" :!type "Texture2D Object Reference"))
  (set `self.Brush Color` (make `LinearColor` (`self.Mask Wetness`) (`self.Mask Snow/Dust`) 0.0 1.0))
  (set `self.Brush Location` (- (`KismetMathLibrary.Conv_VectorToVector2D` (`self.K2_GetActorLocation`)) (/ (`self.Brush Scale`) 2.0)))
  (set `self.Center Location` (`KismetMathLibrary.Conv_VectorToVector2D` (`self.K2_GetActorLocation`)))
  (set `self.Max Distance` (`KismetMathLibrary.Hypotenuse` _returnvalue _returnvalue))
  (for _index (range 4)
    (`KismetArrayLibrary.Array_Add` (`self.Corners`) (+ (`KismetMathLibrary.Conv_VectorToVector2D` (`self.K2_GetActorLocation`)) (`KismetMathLibrary.GetRotated2D` (* (`self.Brush Scale`) (select `int` _index :`0` (-1.0 -1.0) :`1` (1.0 1.0) :`2` (-1.0 1.0) :`3` (1.0 -1.0) :!type "Vector2D Structure")) (`self.Yaw`)))))
  (if (not (`KismetSystemLibrary.IsPackagedForDistribution`))
    (bind _returnvalue_2 (`GameplayStatics.GetActorOfClass` "/Game/Resources/External/Sky/Blueprints/Ultra_Dynamic_Weather.Ultra_Dynamic_Weather_C"))
    (if (not (`/Game/Resources/External/Sky/Blueprints/Ultra_Dynamic_Weather.Runtime` _returnvalue_2))
      (set `/Game/Resources/External/Sky/Blueprints/Ultra_Dynamic_Weather.Editor Mask Target Root` (`self.K2_GetActorLocation`) _returnvalue_2)
      (`/Game/Resources/External/Sky/Blueprints/Ultra_Dynamic_Weather.Initialize Weather Mask Target` _returnvalue_2))))
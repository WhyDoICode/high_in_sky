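; UDS_Cloud_Paint_Container is an Ultra Dynamic Sky helper actor that keeps the sky in step with the presence of a cloud paint container.
; On BeginPlay it finds the sky actor and, if that is already initialized, has it update its painted cloud coverage target.
; When destroyed or removed from the world, it notifies the sky that a container is gone.
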(event `self.ReceiveBeginPlay`
  (bind _returnvalue (`GameplayStatics.GetActorOfClass` "/Game/Resources/External/Sky/Blueprints/Ultra_Dynamic_Sky.Ultra_Dynamic_Sky_C"))
  (`/Engine/EditorBlueprintResources/StandardMacros.IsValid` _returnvalue
    (:`Is Valid`
      (if (`/Game/Resources/External/Sky/Blueprints/Ultra_Dynamic_Sky.Initialized` _returnvalue)
        (`/Game/Resources/External/Sky/Blueprints/Ultra_Dynamic_Sky.Update Painted Cloud Coverage Target` _returnvalue)))))

(event `self.ReceiveEndPlay`
  (params (EndPlayReason :type "EEndPlayReason Enum" :default "Destroyed"))
  (if (`KismetArrayLibrary.Array_Contains` (`|MakeArray` "Destroyed" "RemovedFromWorld" :!type "EEndPlayReason Enum") EndPlayReason)
    (bind _returnvalue (`GameplayStatics.GetActorOfClass` "/Game/Resources/External/Sky/Blueprints/Ultra_Dynamic_Sky.Ultra_Dynamic_Sky_C"))
    (`/Engine/EditorBlueprintResources/StandardMacros.IsValid` _returnvalue
      (:`Is Valid`
        (`/Game/Resources/External/Sky/Blueprints/Ultra_Dynamic_Sky.Notify of Removed Cloud Paint Container` _returnvalue)))))

(fn `UserConstructionScript`)